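; Fast enemy character that follows waypoints and costs the player a life when it reaches the end.
; On BeginPlay it passes the speed from FGEnemyStats to FGAutoMove, and FGWaypointFollower feeds each new destination to that mover.
; On arrival it calls ReduceLife on BP_GameMode and destroys itself.
; OnDeath only prints a placeholder debug string.
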(event `self.ReceiveBeginPlay`
  ;[1 1 1] Set Speed
  (`FGAutoMoveComponent.SetSpeed` (`self.FGAutoMove`) (`FGEnemyStats.GetSpeed` (`self.FGEnemyStats`))))

(event `self.FGWaypointFollower.OnNewDestination`
  (params (destination :type "Vector Structure"))
  ;[1 1 1] Waypoint reached
  (`FGAutoMoveComponent.SetDestination` (`self.FGAutoMove`) destination))

(event `self.FGWaypointFollower.OnDestinationReached`
  ;[1 1 1] Destination Reached
  (bind _asbp_game_mode (cast `/Game/Gameplay/Blueprints/GameModes/BP_GameMode` (`GameplayStatics.GetGameMode`))
    (:`then`
      (`FGGameMode.ReduceLife` _asbp_game_mode))
    (:`CastFailed`
      _))
  (`self.K2_DestroyActor`))

(event `self.OnDeath`
  (`KismetSystemLibrary.PrintString` "Hello"))

(fn `UserConstructionScript`)